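; BP_Boss is a boss enemy actor with a weapon and a melee punch trigger.
; On BeginPlay it assigns its muzzle particle, punch trigger, weapon, and shot and damage sounds to variables; the firing logic is not in this graph.
; When the punch trigger overlaps BP_MyCharacter, it deals fixed damage through PlayerTakeDamage and plays a hurt sound at the world origin.
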(event OnComponentBeginOverlap(PunchTrigger)
  (params (OverlappedComponent :type Primitive%20Component%20Object%20Reference) (OtherActor :type Actor%20Object%20Reference) (OtherComp :type Primitive%20Component%20Object%20Reference) (OtherBodyIndex :type Integer) (bFromSweep :type Boolean) (SweepResult :type Hit%20Result%20Structure%20%28by%20ref%29))
  (bind _asbp_my_character (Utilities|Casting|CastToBP_MyCharacter OtherActor))
  (Class|MyCharacter|PlayerTakeDamage _asbp_my_character 1.0)
  (Audio|PlaySoundatLocation "/Game/Sounds/FX/Player/PlayerTakeDamage.PlayerTakeDamage" "0, 0, 0" "0, 0, 0" 1.0 1.0 0.0 0 0 0))

(event EventBeginPlay
  (Variables|Default|SetfireParticle (Variables|Default|GetMuzzleWeapon))
  (Variables|Default|SetboxTrigger (Variables|Default|GetPunchTrigger))
  (Variables|Default|SetmyWeapon (Variables|Default|GetBossWeapon))
  (Variables|Default|SetfireSound (Variables|Default|GetBossShot))
  (Variables|Default|SetbossDamageSound (Variables|Default|GetBossDamage)))

(fn ConstructionScript)