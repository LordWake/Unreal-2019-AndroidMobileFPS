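; BP_DroneBullet is a drone projectile that freezes the player character on contact.
; On overlap with BP_MyCharacter it sets OnFreeze once, guarded by an AlreadyDamage flag, then calls DestroyThisBullet.
; Overlaps with turrets, freeze drones, lasers and poison lasers are ignored through a cast chain, while any other actor destroys the bullet.
; BeginPlay assigns its death particle and resets the hit flag.
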(event OnComponentBeginOverlap(Bullet)
  (params (OverlappedComponent :type Primitive%20Component%20Object%20Reference) (OtherActor :type Actor%20Object%20Reference) (OtherComp :type Primitive%20Component%20Object%20Reference) (OtherBodyIndex :type Integer) (bFromSweep :type Boolean) (SweepResult :type Hit%20Result%20Structure%20%28by%20ref%29))
  (bind _asbp_my_character (Utilities|Casting|CastToBP_MyCharacter OtherActor)
    (:then
      (if (not (Variables|Default|GetAlreadyDamage))
        (Variables|/Script/BerkeLyum.MyCharacter|SetonFreeze _asbp_my_character true)
        (Variables|Default|SetAlreadyDamage true)
        (Class|DroneBullet|DestroyThisBullet :!label _label)))
    (:CastFailed
      (Utilities|Casting|CastToBP_MyTurret OtherActor
        (:CastFailed
          (Utilities|Casting|CastToBP_FreezeDrone OtherActor
            (:CastFailed
              (Utilities|Casting|CastToBP_Laser OtherActor
                (:CastFailed
                  (Utilities|Casting|CastToBP_PoisonLaser OtherActor
                    (:CastFailed
                      (goto _label))))))))))))

(event EventBeginPlay
  (Utilities|FlowControl|Sequence
    (:then_0
      (Variables|Default|SetdeadParticle (Variables|Default|GetmyDeadParticle)))
    (:then_1
      (Variables|Default|SetAlreadyDamage false))))

(fn ConstructionScript)