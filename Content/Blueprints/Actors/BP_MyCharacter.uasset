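; Player character Blueprint that handles hitscan shooting with a rifle, automatic weapon and shotgun against turrets, freeze drones and the boss.
; BeginPlay fills weapon, muzzle-particle and status-sound references, and the gamepad right trigger calls StartShoot and StopShoot.
; Tick polls two flags, running either one camera trace or a five-trace shotgun cross with fixed world-axis offsets.
; Traces spawn impact particles and damage cast-matched enemies, then each flag resets with a sound.
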(event EventBeginPlay
  (Utilities|FlowControl|Sequence
    (:then_0
      ;[1 0 0.005713] Weapon Mesh
      (Variables|Default|SetmyRifle (Variables|Default|GetGun))
      (Variables|Default|SetmyAutomaticWeapon (Variables|Default|GetMachineGun))
      (Variables|Default|SetmyShotGun (Variables|Default|GetShotGun)))
    (:then_1
      ;[0.09643 1 0] Weapon Muzzle Particles
      (Variables|Default|SetrifleMuzzle (Variables|Default|GetFireParticle))
      (Variables|Default|SetautomaticMuzzle (Variables|Default|GetMachineGunParticle))
      (Variables|Default|SetshotGunMuzzle (Variables|Default|GetShotgunParticle)))
    (:then_2
      (Variables|Default|SetfrozenSound (Variables|Default|GetFrozenEffect_Cue))
      (Variables|Default|SetpoisonSound (Variables|Default|GetPoisonEffect_Cue)))))

(event EventTick
  (params (DeltaSeconds :type Float%20%28single-precision%29))
  (bind _camera (Variables|Default|GetCamera))
  (bind _camera_2 (Variables|Default|GetCamera))
  (bind _returnvalue (Transformation|GetWorldLocation _camera_2))
  (bind _returnvalue_2 (Transformation|GetWorldLocation _camera))
  (bind _returnvalue_3 (Transformation|GetWorldRotation _camera))
  (bind _returnvalue_4 (Math|Vector|GetForwardVector _returnvalue_3))
  (bind _returnvalue_5 (* _returnvalue_4 1e+04))
  (bind _returnvalue_6 (+ _returnvalue_2 _returnvalue_5))
  (Utilities|FlowControl|Sequence
    (:then_0
      ;[1 0.03 0] Shoot Raycast
      (if (Variables|Default|GetmakeARaycast)
        (bind _outhit (Collision|LineTraceByChannel _returnvalue (+ _returnvalue (* (Math|Vector|GetForwardVector (Transformation|GetWorldRotation _camera_2)) 1e+04)) "TraceTypeQuery1" false (Actor|GetAllChildActors true) "None"))
        (Effects|SpawnEmitteratLocation "/Game/SciFiWeapLight/FX/Particles/P_Impact_Metal_Large_Dark.P_Impact_Metal_Large_Dark" (.ImpactPoint (Collision|BreakHitResult _outhit)))
        (bind _asbp_my_turret (Utilities|Casting|CastToBP_MyTurret (.HitActor (Collision|BreakHitResult _outhit)))
          (:then
            (Class|Turret|TakeTurretDamage _asbp_my_turret 1.0))
          (:CastFailed
            (bind _asbp_freeze_drone (Utilities|Casting|CastToBP_FreezeDrone (.HitActor (Collision|BreakHitResult _outhit)))
              (:then
                (Class|FreezeDrone|TakeDroneDamage _asbp_freeze_drone 1.0))
              (:CastFailed
                (bind _asbp_boss (Utilities|Casting|CastToBP_Boss (.HitActor (Collision|BreakHitResult _outhit)))
                  (:then
                    (Class|Boss|TakeBossDamage _asbp_boss 1.0))
                  (:CastFailed
                    _))))))
        (Variables|Default|SetmakeARaycast false)
        (Audio|PlaySoundatLocation "/Game/Sounds/FX/Player/PlayerShot_Cue.PlayerShot_Cue" "0, 0, 0" "0, 0, 0" 1.0 1.0 0.0 0 0 0)))
    (:then_1
      (if (Variables|Default|GetmakeAShotGunRaycast)
        (Utilities|FlowControl|Sequence
          (:then_0
            (bind _outhit_2 (Collision|LineTraceByChannel _returnvalue_2 _returnvalue_6 "TraceTypeQuery1" false 0 "None"))
            (Effects|SpawnEmitteratLocation "/Game/SciFiWeapLight/FX/Particles/P_Impact_Metal_Large_Dark.P_Impact_Metal_Large_Dark" (.ImpactPoint (Collision|BreakHitResult _outhit_2)))
            (bind _asbp_my_turret_2 (Utilities|Casting|CastToBP_MyTurret (.HitActor (Collision|BreakHitResult _outhit_2)))
              (:then
                (Class|Turret|TakeTurretDamage _asbp_my_turret_2 1.0))
              (:CastFailed
                (bind _asbp_freeze_drone_2 (Utilities|Casting|CastToBP_FreezeDrone (.HitActor (Collision|BreakHitResult _outhit_2)))
                  (:then
                    (Class|FreezeDrone|TakeDroneDamage _asbp_freeze_drone_2 1.0))
                  (:CastFailed
                    (bind _asbp_boss_2 (Utilities|Casting|CastToBP_Boss (.HitActor (Collision|BreakHitResult _outhit_2))))
                    (Class|Boss|TakeBossDamage _asbp_boss_2 1.0))))))
          (:then_1
            (bind _outhit_3 (Collision|LineTraceByChannel _returnvalue_2 (+ _returnvalue_6 "50.000000,0.000000,0.000000") "TraceTypeQuery1" false 0 "None"))
            (Effects|SpawnEmitteratLocation "/Game/SciFiWeapLight/FX/Particles/P_Impact_Metal_Large_Dark.P_Impact_Metal_Large_Dark" (.ImpactPoint (Collision|BreakHitResult _outhit_3)))
            (bind _asbp_my_turret_3 (Utilities|Casting|CastToBP_MyTurret (.HitActor (Collision|BreakHitResult _outhit_3)))
              (:then
                (Class|Turret|TakeTurretDamage _asbp_my_turret_3 1.0))
              (:CastFailed
                (bind _asbp_freeze_drone_3 (Utilities|Casting|CastToBP_FreezeDrone (.HitActor (Collision|BreakHitResult _outhit_3)))
                  (:then
                    (Class|FreezeDrone|TakeDroneDamage _asbp_freeze_drone_3 1.0))
                  (:CastFailed
                    (bind _asbp_boss_3 (Utilities|Casting|CastToBP_Boss (.HitActor (Collision|BreakHitResult _outhit_3))))
                    (Class|Boss|TakeBossDamage _asbp_boss_3 1.0))))))
          (:then_2
            (bind _outhit_4 (Collision|LineTraceByChannel _returnvalue_2 (+ _returnvalue_6 "-50.000000,0.000000,0.000000") "TraceTypeQuery1" false 0 "None"))
            (Effects|SpawnEmitteratLocation "/Game/SciFiWeapLight/FX/Particles/P_Impact_Metal_Large_Dark.P_Impact_Metal_Large_Dark" (.ImpactPoint (Collision|BreakHitResult _outhit_4)))
            (bind _asbp_my_turret_4 (Utilities|Casting|CastToBP_MyTurret (.HitActor (Collision|BreakHitResult _outhit_4)))
              (:then
                (Class|Turret|TakeTurretDamage _asbp_my_turret_4 1.0))
              (:CastFailed
                (bind _asbp_freeze_drone_4 (Utilities|Casting|CastToBP_FreezeDrone (.HitActor (Collision|BreakHitResult _outhit_4)))
                  (:then
                    (Class|FreezeDrone|TakeDroneDamage _asbp_freeze_drone_4 1.0))
                  (:CastFailed
                    (bind _asbp_boss_4 (Utilities|Casting|CastToBP_Boss (.HitActor (Collision|BreakHitResult _outhit_4))))
                    (Class|Boss|TakeBossDamage _asbp_boss_4 1.0))))))
          (:then_3
            (bind _outhit_5 (Collision|LineTraceByChannel _returnvalue_2 (+ _returnvalue_6 "0.000000,0.000000,50.000000") "TraceTypeQuery1" false 0 "None"))
            (Effects|SpawnEmitteratLocation "/Game/SciFiWeapLight/FX/Particles/P_Impact_Metal_Large_Dark.P_Impact_Metal_Large_Dark" (.ImpactPoint (Collision|BreakHitResult _outhit_5)))
            (bind _asbp_my_turret_5 (Utilities|Casting|CastToBP_MyTurret (.HitActor (Collision|BreakHitResult _outhit_5)))
              (:then
                (Class|Turret|TakeTurretDamage _asbp_my_turret_5 1.0))
              (:CastFailed
                (bind _asbp_freeze_drone_5 (Utilities|Casting|CastToBP_FreezeDrone (.HitActor (Collision|BreakHitResult _outhit_5)))
                  (:then
                    (Class|FreezeDrone|TakeDroneDamage _asbp_freeze_drone_5 1.0))
                  (:CastFailed
                    (bind _asbp_boss_5 (Utilities|Casting|CastToBP_Boss (.HitActor (Collision|BreakHitResult _outhit_5))))
                    (Class|Boss|TakeBossDamage _asbp_boss_5 1.0))))))
          (:then_4
            (bind _outhit_6 (Collision|LineTraceByChannel _returnvalue_2 (+ _returnvalue_6 "0.000000,0.000000,-50.000000") "TraceTypeQuery1" false 0 "None"))
            (Effects|SpawnEmitteratLocation "/Game/SciFiWeapLight/FX/Particles/P_Impact_Metal_Large_Dark.P_Impact_Metal_Large_Dark" (.ImpactPoint (Collision|BreakHitResult _outhit_6)))
            (bind _asbp_my_turret_6 (Utilities|Casting|CastToBP_MyTurret (.HitActor (Collision|BreakHitResult _outhit_6)))
              (:then
                (Class|Turret|TakeTurretDamage _asbp_my_turret_6 1.0))
              (:CastFailed
                (bind _asbp_freeze_drone_6 (Utilities|Casting|CastToBP_FreezeDrone (.HitActor (Collision|BreakHitResult _outhit_6)))
                  (:then
                    (Class|FreezeDrone|TakeDroneDamage _asbp_freeze_drone_6 1.0))
                  (:CastFailed
                    (bind _asbp_boss_6 (Utilities|Casting|CastToBP_Boss (.HitActor (Collision|BreakHitResult _outhit_6))))
                    (Class|Boss|TakeBossDamage _asbp_boss_6 1.0))))))
          (:then_5
            (Variables|Default|SetmakeAShotGunRaycast false)
            (Audio|PlaySoundatLocation "/Game/Sounds/FX/Player/PlayerShotGun.PlayerShotGun" "0, 0, 0" "0, 0, 0" 1.0 1.0 0.0 0 0 0)))))))

(event Input|GamepadEvents|GamepadRightTrigger
  (params (Key :type Key%20Structure))
  (:Pressed
    (Class|MyCharacter|StartShoot))
  (:Released
    (Class|MyCharacter|StopShoot)))

(fn ConstructionScript)