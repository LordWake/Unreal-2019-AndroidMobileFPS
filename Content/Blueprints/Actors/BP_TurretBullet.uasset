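; BP_TurretBullet is a projectile that deals one-time damage to the player.
; On overlap it damages BP_MyCharacter once, guarded by a flag, plays a hit sound at the world origin and destroys itself.
; A chain of casts lets it ignore turrets, lasers, poison lasers and the boss, while any other actor destroys it.
; BeginPlay assigns its death particle and resets the damage flag.
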(event OnComponentBeginOverlap(Bullet)
  (params (OverlappedComponent :type Primitive%20Component%20Object%20Reference) (OtherActor :type Actor%20Object%20Reference) (OtherComp :type Primitive%20Component%20Object%20Reference) (OtherBodyIndex :type Integer) (bFromSweep :type Boolean) (SweepResult :type Hit%20Result%20Structure%20%28by%20ref%29))
  (bind _asbp_my_character (Utilities|Casting|CastToBP_MyCharacter OtherActor)
    (:then
      (if (not (Variables|Default|GetAlreadyDamage))
        (Class|MyCharacter|PlayerTakeDamage _asbp_my_character 1.0)
        (Variables|Default|SetAlreadyDamage true)
        (Audio|PlaySoundatLocation "/Game/Sounds/FX/Player/PlayerTakeDamage.PlayerTakeDamage" "0, 0, 0" "0, 0, 0" 1.0 1.0 0.0 0 0 0)
        (Class|TurretBullet|DestroyThisBullet :!label _label)))
    (:CastFailed
      (Utilities|Casting|CastToBP_MyTurret OtherActor
        (:CastFailed
          (Utilities|Casting|CastToBP_Laser OtherActor
            (:CastFailed
              (Utilities|Casting|CastToBP_PoisonLaser OtherActor
                (:CastFailed
                  (Utilities|Casting|CastToBP_Boss OtherActor
                    (:CastFailed
                      (goto _label))))))))))))

(event EventBeginPlay
  (Variables|Default|SetdeadParticle (Variables|Default|GetMyDeadParticle))
  (Variables|Default|SetAlreadyDamage false))

(fn ConstructionScript)